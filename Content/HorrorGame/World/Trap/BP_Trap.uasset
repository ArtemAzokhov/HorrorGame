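; BP_Trap is a one-shot trap for the horror game that damages a player-controlled Character.
; When such a Character overlaps its Box, it plays a sound at the trap's location, applies fixed damage, sets a triggered flag and hides its Effect component.
; A temporary walk-speed slowdown with a delayed restore is present but disconnected, so it never runs.
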(event `self.Box.OnComponentBeginOverlap`
  (params (OverlappedComponent :type "PrimitiveComponent Object Reference") (OtherActor :type "Actor Object Reference") (OtherComp :type "PrimitiveComponent Object Reference") (OtherBodyIndex :type Integer) (bFromSweep :type Boolean) (SweepResult :type "HitResult Structure (by ref)"))
  (bind _ascharacter (cast `Character` OtherActor))
  (if (and (`GameplayStatics.ObjectIsA` (`Pawn.GetController` _ascharacter) "/Script/Engine.PlayerController") (not (`self.bIsTrapTriggered`)))
    (`GameplayStatics.PlaySoundAtLocation` (`self.Sound`) (`self.K2_GetActorLocation`) (struct) 1.0 1.0 0.0 null null null null)
    (`GameplayStatics.ApplyDamage` OtherActor 30.0)
    (set `self.bIsTrapTriggered` true)
    (`SceneComponent.SetVisibility` (`self.Effect`) false false)))

(fn `UserConstructionScript`)